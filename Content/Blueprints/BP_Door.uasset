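; BP_Door is a locked door that swings open when the player enters its trigger box holding a key.
; The box overlap casts to BP_ThirdPersonCharacterCustom and, if KeyCount is above zero, spends one key and plays the TL_Door timeline.
; The timeline lerps SMDoor's relative yaw to a quarter turn; without a key it prints a locked message.
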(event `self.Box.OnComponentBeginOverlap`
  (params (OverlappedComponent :type "PrimitiveComponent Object Reference") (OtherActor :type "Actor Object Reference") (OtherComp :type "PrimitiveComponent Object Reference") (OtherBodyIndex :type Integer) (bFromSweep :type Boolean) (SweepResult :type "HitResult Structure (by ref)"))
  (bind _asbp_third_person_character_custom (cast `/Game/Blueprints/BP_ThirdPersonCharacterCustom` OtherActor))
  (bind _keycount (`/Game/Blueprints/BP_ThirdPersonCharacterCustom.KeyCount` _asbp_third_person_character_custom))
  (if (> _keycount 0)
    (set `/Game/Blueprints/BP_ThirdPersonCharacterCustom.KeyCount` (+ _keycount -1) _asbp_third_person_character_custom)
    (bind (_direction _newtrack_0) (`Timeline|TL_Door`)
      (:`Update`
        (`SceneComponent.K2_SetRelativeRotation` (`self.SM_Door`) (`KismetMathLibrary.MakeRotator` 0.0 0.0 (`KismetMathLibrary.Lerp` 0.0 -90.0 _newtrack_0)) false false)))
    (else
      (`KismetSystemLibrary.PrintString` "Door is locked."))))

(fn `UserConstructionScript`)