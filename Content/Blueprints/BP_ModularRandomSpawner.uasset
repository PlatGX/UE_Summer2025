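; BP_ModularRandomSpawner is an actor that spawns a configurable class at a random TargetPoints transform.
; Spawning starts on BeginPlay or, with UseOverlapTrigger, whenever BP_ThirdPersonCharacterCustom overlaps the Box.
; The first spawn is immediate; LoopSpawn then repeats it through a delayed recursive event until LoopSpawnCounter reaches its limit.
; Invalid class or empty points print an error, and random picks can reuse locations.
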(event `StartLoopingSpawn`
  (bind _targetpoints (`self.TargetPoints`))
  ; Loop Spawn
  (if (< (`self.LoopSpawnCounter`) (`self.LoopSpawnLimit`))
    (`/Engine/EditorBlueprintResources/StandardMacros.IncrementInt` (`self.LoopSpawnCounter`)
      (:`  `
        (`KismetSystemLibrary.Delay` (`self.LoopSpawnInterval`))
        ; Validation
        (if (and (`KismetSystemLibrary.IsValidClass` (`self.SpawnClass`)) (`KismetArrayLibrary.Array_IsNotEmpty` _targetpoints)) :!label _label
          ; Spawn Actor
          (`|SpawnActorFromClass` (`self.SpawnClass`) (`self.GetTransform` (`KismetArrayLibrary.Array_Random` _targetpoints)) "Undefined" "MultiplyWithRoot" null null)
          (if (`self.bLoopSpawn`)
            (`self.StartLoopingSpawn`))
          (else
            (`KismetSystemLibrary.PrintString` "BP_ModularRandomSpawner failed to validate the variables." true true (struct :`R` 1.0 :`A` 1.0) 5.0)))))))

(event `self.ReceiveBeginPlay`
  ; Start spawning on begin play or on box collision?
  (if (not (`self.bUseOverlapTrigger`))
    (`self.StartSpawn`)))

(event `StartSpawn`
  ; Validation
  (goto _label))

(event `self.Box.OnComponentBeginOverlap`
  (params (OverlappedComponent :type "PrimitiveComponent Object Reference") (OtherActor :type "Actor Object Reference") (OtherComp :type "PrimitiveComponent Object Reference") (OtherBodyIndex :type Integer) (bFromSweep :type Boolean) (SweepResult :type "HitResult Structure (by ref)"))
  ; Start spawning on begin play or on box collision?
  (cast `/Game/Blueprints/BP_ThirdPersonCharacterCustom` OtherActor)
  (if (`self.bUseOverlapTrigger`)
    (`self.StartSpawn`)))

(fn `UserConstructionScript`)