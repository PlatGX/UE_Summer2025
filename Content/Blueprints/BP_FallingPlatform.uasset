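; A platform that falls shortly after the player character enters its trigger box, then returns and re-arms.
; Activate, Drop and Reset run in sequence: a delayed physics drop, then a timeline-driven transform lerp back to the BeginPlay pose.
; Timelines blend scalar material parameters to color each stage, zeroed when IsReady is restored.
; The stage delays and follow-on calls hang off timeline Update pins rather than Finished, except after the return move.
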(event `self.ReceiveBeginPlay`
  (set `self.StartingTransform` (`SceneComponent.K2_GetComponentToWorld` (`self.Cube`)))
  (`PrimitiveComponent.SetMaterial` (`self.Cube`) 0 "/Game/Materials/ModularLerpingMaterial.ModularLerpingMaterial"))

(event `self.Box.OnComponentBeginOverlap`
  (params (OverlappedComponent :type "PrimitiveComponent Object Reference") (OtherActor :type "Actor Object Reference") (OtherComp :type "PrimitiveComponent Object Reference") (OtherBodyIndex :type Integer) (bFromSweep :type Boolean) (SweepResult :type "HitResult Structure (by ref)"))
  (cast `/Game/Blueprints/BP_ThirdPersonCharacterCustom` OtherActor)
  (`self.Activate`))

(event `Activate`
  (if (`self.bIsReady`)
    (`KismetSystemLibrary.PrintString` "One Second Left")
    (set `self.bIsReady` false)
    (bind (_direction _colorinterpolation) (`Timeline|Timeline` :!via `PlayFromStart`)
      (:`Update`
        (`MeshComponent.SetScalarParameterValueOnMaterials` (`self.Cube`) "OneToTwo" _colorinterpolation)
        (`KismetSystemLibrary.Delay` 1.0)
        (`self.Drop`)))
    (else
      (`KismetSystemLibrary.PrintString` "not ready"))))

(event `Drop`
  (`KismetSystemLibrary.PrintString` "Drop")
  (bind (_direction _colorinterpolation) (`Timeline|Timeline_0` :!via `PlayFromStart`)
    (:`Update`
      (`MeshComponent.SetScalarParameterValueOnMaterials` (`self.Cube`) "TwoToThree" _colorinterpolation)
      (`PrimitiveComponent.SetSimulatePhysics` (`self.Cube`) true)
      (`KismetSystemLibrary.Delay` 3.0)
      (`self.Reset`))))

(event `Reset`
  (`KismetSystemLibrary.PrintString` "Resetting")
  (set `self.ResetTransform` (`SceneComponent.K2_GetComponentToWorld` (`self.Cube`)))
  (`PrimitiveComponent.SetSimulatePhysics` (`self.Cube`) false)
  (bind (_direction _colorinterpolation) (`Timeline|Timeline_1` :!via `PlayFromStart`)
    (:`Update`
      (`MeshComponent.SetScalarParameterValueOnMaterials` (`self.Cube`) "ThreeToFour" _colorinterpolation)
      (bind (_direction_2 _newtrack_0) (`Timeline|GoBackToStart` :!via `PlayFromStart`)
        (:`Update`
          (bind (_returnvalue_location _returnvalue_rotation) (`KismetMathLibrary.BreakTransform` (`KismetMathLibrary.TLerp` (`self.ResetTransform`) (`self.StartingTransform`) _newtrack_0)))
          (`SceneComponent.K2_SetWorldLocationAndRotation` (`self.Cube`) _returnvalue_location _returnvalue_rotation false false))
        (:`Finished`
          (bind (_direction_3 _colorinterpolation_2) (`Timeline|Timeline_2` :!via `PlayFromStart`)
            (:`Update`
              (`MeshComponent.SetScalarParameterValueOnMaterials` (`self.Cube`) "FourToOne" _colorinterpolation_2)
              (`KismetSystemLibrary.Delay` 1.0)
              (set `self.bIsReady` true)
              (`MeshComponent.SetScalarParameterValueOnMaterials` (`self.Cube`) "OneToTwo" 0.0)
              (`MeshComponent.SetScalarParameterValueOnMaterials` (`self.Cube`) "TwoToThree" 0.0)
              (`MeshComponent.SetScalarParameterValueOnMaterials` (`self.Cube`) "ThreeToFour" 0.0)
              (`MeshComponent.SetScalarParameterValueOnMaterials` (`self.Cube`) "FourToOne" 0.0))))))))

(fn `UserConstructionScript`)